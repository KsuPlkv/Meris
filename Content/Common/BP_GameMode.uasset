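; Game mode for a falling-block game that shows the main UI and spawns new figures.
; On BeginPlay it creates WB_Main, stores it and adds it to the viewport.
; SpawnBlocks picks a random entry from FiguresExamples, spawns an actor of that class at the spawn point and triggers its falling event as a BP_Figure.
; Nothing in this Blueprint calls SpawnBlocks, and Tick is unused.
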(event EventBeginPlay
  (bind _returnvalue (UserInterface|CreateWidget "/Game/UI/WB_Main.WB_Main_C" (Game|GetPlayerController 0)))
  (bind _output_get (Variables|Default|SetW_main _returnvalue))
  (UserInterface|Viewport|AddtoViewport _output_get 0))

(event EventTick
  (params (DeltaSeconds :type Float%20%28single-precision%29)))

(fn ConstructionScript)

(fn SpawnBlocks
  (bind _returnvalue (Game|SpawnActorfromClass (Utilities|GetClass (.OutItem (Utilities|Array|Random (Variables|Default|GetFiguresExamples)))) (Math|Transform|MakeTransform (Transformation|GetWorldLocation (Variables|/Game/Actors/BP_SpawnPoint.BP_SpawnPoint_C|GetDefaultSceneRoot (Variables|Default|GetSpawnPoin))) "0, 0, 0" "1.000000,1.000000,1.000000") "Undefined" "MultiplyWithRoot" 0 0))
  (bind _output_get (Variables|Default|SetNewBlock _returnvalue))
  (Default|OnFallingEvent (.AsBP%20Figure (Utilities|Casting|CastToBP_Figure _output_get)) _output_get))