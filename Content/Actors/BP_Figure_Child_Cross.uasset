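; Cross-shaped figure piece, by its name a BP_Figure child, built from five meshes and five collision boxes for a block-placement game.
; The paint event applies the parent material to every mesh.
; Any box overlapping BP_Field flags the GameMode's NewBlock as overlapping the frame; two boxes start with collision disabled.
; The end event enables query collision on all boxes, marks the piece ended and gathers unique overlapped BP_CollisionCells.
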(event OnComponentBeginOverlap(Box3)
  (params (OverlappedComponent :type Primitive%20Component%20Object%20Reference) (OtherActor :type Actor%20Object%20Reference) (OtherComp :type Primitive%20Component%20Object%20Reference) (OtherBodyIndex :type Integer) (bFromSweep :type Boolean) (SweepResult :type Hit%20Result%20Structure%20%28by%20ref%29))
  (Utilities|Casting|CastToBP_Field OtherActor)
  (Variables|/Game/Actors/BP_Figure.BP_Figure_C|SetIsOverlappedFrame (.AsBP%20Figure (Utilities|Casting|CastToBP_Figure (Variables|/Game/Common/BP_GameMode.BP_GameMode_C|GetNewBlock (.AsBP%20Game%20Mode (Utilities|Casting|CastToBP_GameMode (Game|GetGameMode)))))) true))

(event OnComponentBeginOverlap(Box4)
  (params (OverlappedComponent :type Primitive%20Component%20Object%20Reference) (OtherActor :type Actor%20Object%20Reference) (OtherComp :type Primitive%20Component%20Object%20Reference) (OtherBodyIndex :type Integer) (bFromSweep :type Boolean) (SweepResult :type Hit%20Result%20Structure%20%28by%20ref%29))
  (Utilities|Casting|CastToBP_Field OtherActor)
  (Variables|/Game/Actors/BP_Figure.BP_Figure_C|SetIsOverlappedFrame (.AsBP%20Figure (Utilities|Casting|CastToBP_Figure (Variables|/Game/Common/BP_GameMode.BP_GameMode_C|GetNewBlock (.AsBP%20Game%20Mode (Utilities|Casting|CastToBP_GameMode (Game|GetGameMode)))))) true))

(event OnComponentBeginOverlap(Box6)
  (params (OverlappedComponent :type Primitive%20Component%20Object%20Reference) (OtherActor :type Actor%20Object%20Reference) (OtherComp :type Primitive%20Component%20Object%20Reference) (OtherBodyIndex :type Integer) (bFromSweep :type Boolean) (SweepResult :type Hit%20Result%20Structure%20%28by%20ref%29))
  (Utilities|Casting|CastToBP_Field OtherActor)
  (Variables|/Game/Actors/BP_Figure.BP_Figure_C|SetIsOverlappedFrame (.AsBP%20Figure (Utilities|Casting|CastToBP_Figure (Variables|/Game/Common/BP_GameMode.BP_GameMode_C|GetNewBlock (.AsBP%20Game%20Mode (Utilities|Casting|CastToBP_GameMode (Game|GetGameMode)))))) true))

(event OnComponentBeginOverlap(Box5)
  (params (OverlappedComponent :type Primitive%20Component%20Object%20Reference) (OtherActor :type Actor%20Object%20Reference) (OtherComp :type Primitive%20Component%20Object%20Reference) (OtherBodyIndex :type Integer) (bFromSweep :type Boolean) (SweepResult :type Hit%20Result%20Structure%20%28by%20ref%29))
  (Utilities|Casting|CastToBP_Field OtherActor)
  (Variables|/Game/Actors/BP_Figure.BP_Figure_C|SetIsOverlappedFrame (.AsBP%20Figure (Utilities|Casting|CastToBP_Figure (Variables|/Game/Common/BP_GameMode.BP_GameMode_C|GetNewBlock (.AsBP%20Game%20Mode (Utilities|Casting|CastToBP_GameMode (Game|GetGameMode)))))) true))

(event OnComponentBeginOverlap(Box)
  (params (OverlappedComponent :type Primitive%20Component%20Object%20Reference) (OtherActor :type Actor%20Object%20Reference) (OtherComp :type Primitive%20Component%20Object%20Reference) (OtherBodyIndex :type Integer) (bFromSweep :type Boolean) (SweepResult :type Hit%20Result%20Structure%20%28by%20ref%29))
  (Utilities|Casting|CastToBP_Field OtherActor)
  (Variables|/Game/Actors/BP_Figure.BP_Figure_C|SetIsOverlappedFrame (.AsBP%20Figure (Utilities|Casting|CastToBP_Figure (Variables|/Game/Common/BP_GameMode.BP_GameMode_C|GetNewBlock (.AsBP%20Game%20Mode (Utilities|Casting|CastToBP_GameMode (Game|GetGameMode)))))) true))

(event Custom|SetMat
  (for _array_element (Variables|Default|GetMeshes)
    (Rendering|Material|SetMaterial _array_element 0 (Variables|Default|GetParentMaterial))))

(event Custom|CustomEvent
  (CallFunction|FSetBlock))

(event EventBeginPlay
  (bind _meshes (Variables|Default|GetMeshes))
  (|CallParentFunction)
  (Utilities|Array|Add _meshes (Variables|Default|GetStaticMesh4))
  (Utilities|Array|Add _meshes (Variables|Default|GetStaticMesh3))
  (Utilities|Array|Add _meshes (Variables|Default|GetStaticMesh2))
  (Utilities|Array|Add _meshes (Variables|Default|GetStaticMesh1))
  (Utilities|Array|Add _meshes (Variables|Default|GetStaticMesh))
  (Variables|Default|SetIsEnd false)
  (Collision|SetCollisionEnabled (Variables|Default|GetBox5) "NoCollision")
  (EventDispatchers|BindEventtoOnPaint (delegate Custom|SetMat))
  (EventDispatchers|BindEventtoOnEnd (delegate Custom|CustomEvent)))

(fn ConstructionScript
  (|CallParentFunction))

(fn FSetBlock
  (bind _box4 (Variables|Default|GetBox4))
  (Collision|SetCollisionEnabled _box4 "QueryOnly")
  (Variables|Default|SetIsEnd true)
  (for _array_element (Collision|GetOverlappingActors _box4 "/Game/Actors/BP_CollisionCell.BP_CollisionCell_C" :!class /Script/Engine.PrimitiveComponent)
    (bind _asbp_collision_cell (Utilities|Casting|CastToBP_CollisionCell _array_element))
    (Utilities|Array|AddUnique (Variables|Default|GetOverlappedCells) _asbp_collision_cell))
  (for _array_element_2 (Collision|GetOverlappingActors (Variables|Default|GetBox3) "/Game/Actors/BP_CollisionCell.BP_CollisionCell_C" :!class /Script/Engine.PrimitiveComponent)
    (bind _asbp_collision_cell_2 (Utilities|Casting|CastToBP_CollisionCell _array_element_2))
    (Utilities|Array|AddUnique (Variables|Default|GetOverlappedCells) _asbp_collision_cell_2))
  (for _array_element_3 (Collision|GetOverlappingActors (Variables|Default|GetBox6) "/Game/Actors/BP_CollisionCell.BP_CollisionCell_C" :!class /Script/Engine.PrimitiveComponent)
    (bind _asbp_collision_cell_3 (Utilities|Casting|CastToBP_CollisionCell _array_element_3))
    (Utilities|Array|AddUnique (Variables|Default|GetOverlappedCells) _asbp_collision_cell_3))
  (for _array_element_4 (Collision|GetOverlappingActors (Variables|Default|GetBox5) "/Game/Actors/BP_CollisionCell.BP_CollisionCell_C" :!class /Script/Engine.PrimitiveComponent)
    (bind _asbp_collision_cell_4 (Utilities|Casting|CastToBP_CollisionCell _array_element_4))
    (Utilities|Array|AddUnique (Variables|Default|GetOverlappedCells) _asbp_collision_cell_4))
  (for _array_element_5 (Collision|GetOverlappingActors (Variables|Default|GetBox) "/Game/Actors/BP_CollisionCell.BP_CollisionCell_C" :!class /Script/Engine.PrimitiveComponent)
    (bind _asbp_collision_cell_5 (Utilities|Casting|CastToBP_CollisionCell _array_element_5))
    (Utilities|Array|AddUnique (Variables|Default|GetOverlappedCells) _asbp_collision_cell_5)))