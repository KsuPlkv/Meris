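; BP_Figure_Child_MiniCorner is a child figure Blueprint, apparently the mini-corner shape, made of four static mesh parts that are repainted together.
; On BeginPlay it runs the parent logic, adds the four meshes to a Meshes array and binds SetMat to the OnPaint event.
; SetMat loops over the array and applies ParentMaterial to the first material slot of each mesh.
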(event Custom|SetMat
  (for _array_element (Variables|Default|GetMeshes)
    (Rendering|Material|SetMaterial _array_element 0 (Variables|Default|GetParentMaterial))))

(event EventBeginPlay
  (bind _meshes (Variables|Default|GetMeshes))
  (|CallParentFunction)
  (Utilities|Array|Add _meshes (Variables|Default|GetStaticMesh3))
  (Utilities|Array|Add _meshes (Variables|Default|GetStaticMesh2))
  (Utilities|Array|Add _meshes (Variables|Default|GetStaticMesh1))
  (Utilities|Array|Add _meshes (Variables|Default|GetStaticMesh))
  (EventDispatchers|BindEventtoOnPaint (delegate Custom|SetMat)))

(fn ConstructionScript
  (|CallParentFunction))