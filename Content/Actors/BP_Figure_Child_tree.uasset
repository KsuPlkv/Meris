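; Child figure Blueprint for the "tree" shape, built from three meshes and three collision boxes on top of a parent figure class.
; It binds to the parent's paint, rotation and end events, applying the parent's material to its meshes when painted.
; On rotation, the roll angle selects which boxes have query collision.
; On end, it enables all boxes, sets IsEnd and collects the overlapped BP_CollisionCell actors without duplicates.
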(event Custom|SetMat
  (for _array_element (Variables|Default|GetMeshes)
    (Rendering|Material|SetMaterial _array_element 0 (Variables|Default|GetParentMaterial))))

(event Custom|ChangeRotation
  (CallFunction|FCheckRotation))

(event Custom|CustomEvent
  (CallFunction|FSetBlock))

(event EventBeginPlay
  (bind _meshes (Variables|Default|GetMeshes))
  (|CallParentFunction)
  (Utilities|Array|Add _meshes (Variables|Default|GetStaticMesh2))
  (Utilities|Array|Add _meshes (Variables|Default|GetStaticMesh1))
  (Utilities|Array|Add _meshes (Variables|Default|GetStaticMesh))
  (Variables|Default|SetIsEnd false)
  (EventDispatchers|BindEventtoOnPaint (delegate Custom|SetMat))
  (EventDispatchers|BindEventtoOnRotation (delegate Custom|ChangeRotation))
  (EventDispatchers|BindEventtoOnEnd (delegate Custom|CustomEvent)))

(event Collision|EventActorBeginOverlap
  (params (OtherActor :type Actor%20Object%20Reference)))

(event EventTick
  (params (DeltaSeconds :type Float%20%28single-precision%29)))

(fn ConstructionScript
  (|CallParentFunction))

(fn FCheckRotation
  (bind _returnvalue (Transformation|GetActorRotation))
  (if (== (.roll _returnvalue) 0.0)
    (Collision|SetCollisionEnabled (Variables|Default|GetBox) "QueryOnly")
    (elif (== (.roll _returnvalue) 9e+01)
      (Collision|SetCollisionEnabled (Variables|Default|GetBox) "NoCollision")
      (Collision|SetCollisionEnabled (Variables|Default|GetBox1) "QueryOnly")
      (elif (== (.roll _returnvalue) 1.8e+02)
        (Collision|SetCollisionEnabled (Variables|Default|GetBox) "QueryOnly")
        (elif (== (.roll _returnvalue) -9e+01)
          (Collision|SetCollisionEnabled (Variables|Default|GetBox) "NoCollision")
          (Collision|SetCollisionEnabled (Variables|Default|GetBox2) "QueryOnly"))))))

(fn FSetBlock
  (Collision|SetCollisionEnabled (Variables|Default|GetBox) "QueryOnly")
  (Variables|Default|SetIsEnd true)
  (for _array_element (Collision|GetOverlappingActors (Variables|Default|GetBox2) "/Game/Actors/BP_CollisionCell.BP_CollisionCell_C" :!class /Script/Engine.PrimitiveComponent)
    (bind _asbp_collision_cell (Utilities|Casting|CastToBP_CollisionCell _array_element))
    (Utilities|Array|AddUnique (Variables|Default|GetOverlappedCells) _asbp_collision_cell))
  (for _array_element_2 (Collision|GetOverlappingActors (Variables|Default|GetBox1) "/Game/Actors/BP_CollisionCell.BP_CollisionCell_C" :!class /Script/Engine.PrimitiveComponent)
    (bind _asbp_collision_cell_2 (Utilities|Casting|CastToBP_CollisionCell _array_element_2))
    (Utilities|Array|AddUnique (Variables|Default|GetOverlappedCells) _asbp_collision_cell_2))
  (for _array_element_3 (Collision|GetOverlappingActors (Variables|Default|GetBox) "/Game/Actors/BP_CollisionCell.BP_CollisionCell_C" :!class /Script/Engine.PrimitiveComponent)
    (bind _asbp_collision_cell_3 (Utilities|Casting|CastToBP_CollisionCell _array_element_3))
    (Utilities|Array|AddUnique (Variables|Default|GetOverlappedCells) _asbp_collision_cell_3)))