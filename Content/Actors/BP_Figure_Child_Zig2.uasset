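; Child figure Blueprint for a "Zig2" block piece made of four meshes and four collision boxes, apparently for a Tetris-style grid game.
; It binds to paint, rotation and end events, applying the parent material to every mesh on paint.
; Rotation toggles which boxes have query collision based on actor roll in quarter turns.
; On end, it enables all boxes, sets IsEnd and collects overlapped BP_CollisionCell actors into OverlappedCells.
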(event Custom|SetMat
  (for _array_element (Variables|Default|GetMeshes)
    (Rendering|Material|SetMaterial _array_element 0 (Variables|Default|GetParentMaterial))))

(event Custom|ChangeRotation
  (CallFunction|FRotation))

(event Custom|CustomEvent
  (CallFunction|FSetBlock))

(event EventBeginPlay
  (bind _meshes (Variables|Default|GetMeshes))
  (|CallParentFunction)
  (Utilities|Array|Add _meshes (Variables|Default|GetStaticMesh3))
  (Utilities|Array|Add _meshes (Variables|Default|GetStaticMesh))
  (Utilities|Array|Add _meshes (Variables|Default|GetStaticMesh2))
  (Utilities|Array|Add _meshes (Variables|Default|GetStaticMesh1))
  (Variables|Default|SetIsEnd false)
  (Collision|SetCollisionEnabled (Variables|Default|GetBox3) "NoCollision")
  (EventDispatchers|BindEventtoOnPaint (delegate Custom|SetMat))
  (EventDispatchers|BindEventtoOnRotation (delegate Custom|ChangeRotation))
  (EventDispatchers|BindEventtoOnEnd (delegate Custom|CustomEvent)))

(fn ConstructionScript
  (|CallParentFunction))

(fn FSetBlock
  (Collision|SetCollisionEnabled (Variables|Default|GetBox) "QueryOnly")
  (Variables|Default|SetIsEnd true)
  (for _array_element (Collision|GetOverlappingActors (Variables|Default|GetBox3) "/Game/Actors/BP_CollisionCell.BP_CollisionCell_C" :!class /Script/Engine.PrimitiveComponent)
    (bind _asbp_collision_cell (Utilities|Casting|CastToBP_CollisionCell _array_element))
    (Utilities|Array|AddUnique (Variables|Default|GetOverlappedCells) _asbp_collision_cell))
  (for _array_element_2 (Collision|GetOverlappingActors (Variables|Default|GetBox2) "/Game/Actors/BP_CollisionCell.BP_CollisionCell_C" :!class /Script/Engine.PrimitiveComponent)
    (bind _asbp_collision_cell_2 (Utilities|Casting|CastToBP_CollisionCell _array_element_2))
    (Utilities|Array|AddUnique (Variables|Default|GetOverlappedCells) _asbp_collision_cell_2))
  (for _array_element_3 (Collision|GetOverlappingActors (Variables|Default|GetBox1) "/Game/Actors/BP_CollisionCell.BP_CollisionCell_C" :!class /Script/Engine.PrimitiveComponent)
    (bind _asbp_collision_cell_3 (Utilities|Casting|CastToBP_CollisionCell _array_element_3))
    (Utilities|Array|AddUnique (Variables|Default|GetOverlappedCells) _asbp_collision_cell_3))
  (for _array_element_4 (Collision|GetOverlappingActors (Variables|Default|GetBox) "/Game/Actors/BP_CollisionCell.BP_CollisionCell_C" :!class /Script/Engine.PrimitiveComponent)
    (bind _asbp_collision_cell_4 (Utilities|Casting|CastToBP_CollisionCell _array_element_4))
    (Utilities|Array|AddUnique (Variables|Default|GetOverlappedCells) _asbp_collision_cell_4)))

(fn FRotation
  (bind _returnvalue (Transformation|GetActorRotation))
  (if (== (.roll _returnvalue) 0.0)
    (Collision|SetCollisionEnabled (Variables|Default|GetBox1) "QueryOnly")
    (Collision|SetCollisionEnabled (Variables|Default|GetBox3) "NoCollision")
    (elif (== (.roll _returnvalue) 9e+01)
      (Collision|SetCollisionEnabled (Variables|Default|GetBox) "NoCollision")
      (Collision|SetCollisionEnabled (Variables|Default|GetBox3) "QueryOnly")
      (elif (== (.roll _returnvalue) 1.8e+02)
        (Collision|SetCollisionEnabled (Variables|Default|GetBox2) "QueryOnly")
        (Collision|SetCollisionEnabled (Variables|Default|GetBox) "NoCollision")
        (elif (== (.roll _returnvalue) -9e+01)
          (Collision|SetCollisionEnabled (Variables|Default|GetBox1) "NoCollision")
          (Collision|SetCollisionEnabled (Variables|Default|GetBox2) "QueryOnly"))))))