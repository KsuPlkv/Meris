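; BP_CollisionCell is a cell actor with a Box collider that tracks whether a BP_Figure occupies it.
; On BeginPlay it adds itself uniquely to the Cells array on BP_GameMode.
; Box overlap begin and end events from BP_Figure actors set and clear IsEngaged.
; Hovering the cursor over the box only prints a debug "hit" string.
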(event OnComponentBeginOverlap(Box)
  (params (OverlappedComponent :type Primitive%20Component%20Object%20Reference) (OtherActor :type Actor%20Object%20Reference) (OtherComp :type Primitive%20Component%20Object%20Reference) (OtherBodyIndex :type Integer) (bFromSweep :type Boolean) (SweepResult :type Hit%20Result%20Structure%20%28by%20ref%29))
  (Utilities|Casting|CastToBP_Figure OtherActor)
  (Variables|Default|SetIsEngaged true))

(event OnComponentEndOverlap(Box)
  (params (OverlappedComponent :type Primitive%20Component%20Object%20Reference) (OtherActor :type Actor%20Object%20Reference) (OtherComp :type Primitive%20Component%20Object%20Reference) (OtherBodyIndex :type Integer))
  (Utilities|Casting|CastToBP_Figure OtherActor)
  (Variables|Default|SetIsEngaged false))

(event OnBeginCursorOver(Box)
  (params (TouchedComponent :type Primitive%20Component%20Object%20Reference))
  (Development|PrintString "hit"))

(event EventBeginPlay
  (Utilities|Array|AddUnique (Variables|/Game/Common/BP_GameMode.BP_GameMode_C|GetCells (.AsBP%20Game%20Mode (Utilities|Casting|CastToBP_GameMode (Game|GetGameMode)))) self))

(fn ConstructionScript)