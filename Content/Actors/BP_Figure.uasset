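; BP_Figure is a falling block figure on a Tetris-like cell grid that registers its child actors with BP_GameMode.
; Its falling event checks cells below OverlappedCells, then moves down a row and retriggers, or requests new blocks.
; Left/Right input shifts BlockColumn and snaps the actor to the matching game mode cell.
; The overlap event is empty, older collision-driven fall logic is disconnected, and nothing here fills OverlappedCells.
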(event OnComponentBeginOverlap(Box)
  (params (OverlappedComponent :type Primitive%20Component%20Object%20Reference) (OtherActor :type Actor%20Object%20Reference) (OtherComp :type Primitive%20Component%20Object%20Reference) (OtherBodyIndex :type Integer) (bFromSweep :type Boolean) (SweepResult :type Hit%20Result%20Structure%20%28by%20ref%29)))

(event Custom|OnFalling_Event
  (params (Block :type Actor%20Object%20Reference))
  (bind _as_bp_game_mode (Variables|Default|GetAs%20BP%20Game%20Mode))
  (bind _overlappedcells (Variables|Default|GetOverlappedCells))
  (bind _output (Utilities|Array|Get(acopy) _overlappedcells))
  (bind _cells (Variables|/Game/Common/BP_GameMode.BP_GameMode_C|GetCells _as_bp_game_mode))
  (bind _array_element (Utilities|Array|ForEachLoopwithBreak _overlappedcells :!label _label)
    (:LoopBody
      (bind _array_element_2 (Utilities|Array|ForEachLoopwithBreak _cells)
        (:LoopBody
          (if (== (Variables|/Game/Actors/BP_CollisionCell.BP_CollisionCell_C|GetRow _array_element_2) (- (Variables|/Game/Actors/BP_CollisionCell.BP_CollisionCell_C|GetRow _array_element) 1))
            (if (and (Variables|/Game/Actors/BP_CollisionCell.BP_CollisionCell_C|GetIsEngaged _array_element_2) (> (Variables|/Game/Actors/BP_CollisionCell.BP_CollisionCell_C|GetRow _array_element_2) 1))
              (Variables|Default|SetIsRowFree true)
              (else
                (Variables|Default|SetIsRowFree false)
                (goto _label Break)))))))
    (:Completed
      (if (Variables|Default|GetIsRowFree)
        (bind _array_element_3 (Utilities|Array|ForEachLoopwithBreak _cells :!label _label_2)
          (:LoopBody
            (if (and (== (Variables|/Game/Actors/BP_CollisionCell.BP_CollisionCell_C|GetColumn _output) (Variables|/Game/Actors/BP_CollisionCell.BP_CollisionCell_C|GetColumn _array_element_3)) (== (- (Variables|/Game/Actors/BP_CollisionCell.BP_CollisionCell_C|GetRow _output) 1) (Variables|/Game/Actors/BP_CollisionCell.BP_CollisionCell_C|GetRow _array_element_3)))
              (Variables|Default|SetNewLocationCell _array_element_3)
              (goto _label_2 Break)))
          (:Completed
            (Transformation|SetActorLocation (Transformation|GetActorLocation (Variables|Default|GetNewLocationCell)) false false)
            (Variables|Default|SetIsRowFree false)
            (Variables|Default|SetNewLocationCell 0)
            (CallFunction|OnFallingEvent self)))
        (else
          (Default|SpawnBlocks (.AsBP%20Game%20Mode (Utilities|Casting|CastToBP_GameMode (Game|GetGameMode)))))))))

(event Custom|Left/Right
  (params (Value :type Integer))
  (Variables|Default|SetBlockColumn (+ (Variables|Default|GetBlockColumn) Value))
  (bind _array_element (Utilities|Array|ForEachLoopwithBreak (Variables|/Game/Common/BP_GameMode.BP_GameMode_C|GetCells (.AsBP%20Game%20Mode (Utilities|Casting|CastToBP_GameMode (Game|GetGameMode)))) :!label _label)
    (:LoopBody
      (if (and (== (Variables|/Game/Actors/BP_CollisionCell.BP_CollisionCell_C|GetColumn _array_element) (Variables|Default|GetBlockColumn)) (== (Variables|/Game/Actors/BP_CollisionCell.BP_CollisionCell_C|GetRow _array_element) (Variables|Default|GetBlockRow)))
        (Variables|Default|SetNewLocationCell _array_element)
        (goto _label Break)))
    (:Completed
      (if (Variables|Default|GetIsStopped)
        (Variables|Default|SetIsStopped false)
        (Variables|Default|SetNewLocationCell 0)
        (else
          (Utilities|IsValid (Variables|Default|GetNewLocationCell)
            (:Is%20Valid
              (Transformation|SetActorLocation (Transformation|GetActorLocation (Variables|Default|GetNewLocationCell)) true false)
              (Variables|Default|SetBlockColumn (Variables|/Game/Actors/BP_CollisionCell.BP_CollisionCell_C|GetColumn (Variables|Default|GetNewLocationCell)))))))
      (CallFunction|OnFallingEvent self))))

(event EventBeginPlay
  (bind _returnvalue (Game|GetGameMode))
  (bind _asbp_game_mode (Utilities|Casting|CastToBP_GameMode _returnvalue))
  (Variables|Default|SetAs%20BP%20Game%20Mode _asbp_game_mode)
  (for _array_element (Actor|GetAllChildActors true)
    (Utilities|Array|AddUnique (Variables|/Game/Common/BP_GameMode.BP_GameMode_C|GetFiguresExamples _asbp_game_mode) _array_element))
  (Variables|Default|SetBlockColumn 6)
  (Utilities|Array|Clear (Variables|Default|GetOverlappedCells)))

(fn ConstructionScript)